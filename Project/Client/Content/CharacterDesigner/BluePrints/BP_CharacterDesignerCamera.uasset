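; Camera actor for the character designer that zooms between a full-body view and a face view when F is pressed.
; A PositionChange timeline plays or reverses, lerping the root between the BodyPos and FacePos actors while slowing the CharacterDesigner's time dilation toward the face view.
; A Delay-based per-frame loop, started from BeginPlay, repositions FacePos from the character's Head socket plus a UI slider height offset, following body scaling.
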(event `Key|F`
  (params (Key :type "Key Structure" :default "AnyKey"))
  ;[1 1 1] Adjusts Camera Position
  ;;[1 1 1] Sooms in and out
  (:`Pressed`
    (bind _isa (`/Engine/EditorBlueprintResources/StandardMacros.FlipFlop`)
      (:`A`
        (set `self.ZoomedIn?` _isa)
        (bind (_direction _lerppos) (`Timeline|position change` :!label _label)
          (:`Update`
            (set `self.LerpPos` _lerppos)
            (`SceneComponent.K2_SetWorldLocation` (`self.DefaultSceneRoot`) (`KismetMathLibrary.VLerp` (`self.K2_GetActorLocation` (`self.BodyPos`)) (`self.K2_GetActorLocation` (`self.FacePos`)) (`self.LerpPos`)) false false)
            (set `Actor.CustomTimeDilation` (`KismetMathLibrary.Lerp` 1.0 0.5 (`self.LerpPos`)) (`self.CharacterDesigner`)))))
      (:`B`
        (set `self.ZoomedIn?` _isa)
        (goto _label :!via `Reverse`)))))

(event `BeginTick`
  ;[1 1 1] Adjusts Camera Position
  ;;[1 1 1] Updates the location of Face Position so that the camera can lerp to the right location when the body is scaled
  (`self.K2_SetActorRelativeLocation` (`self.FacePos`) (+ (- (`SceneComponent.GetSocketLocation` (`/Game/CharacterDesigner/BluePrints/BP_CharacterDesigner.CustomCharacter` (`self.CharacterDesigner`)) "Head") (-10.0 -40.0 -15.0)) (`KismetMathLibrary.MakeVector` 0.0 0.0 (* (`self.HeightAdjust`) (* (- (`Slider.GetValue` (`/Game/CharacterDesigner/BluePrints/BP_Widget_CharacterDesigner.Slider_CamHeight` (`self.Widget`))) 0.5) 2.0)))) false false :!label _label_2)
  (`KismetSystemLibrary.Delay` (`GameplayStatics.GetWorldDeltaSeconds`))
  (goto _label_2))

(event `self.ReceiveBeginPlay`
  (`KismetSystemLibrary.Delay` 0.01)
  (set `self.Widget` (`/Game/CharacterDesigner/BluePrints/BP_CharacterDesigner.CharacterDesignerUI` (`self.CharacterDesigner`)))
  (`self.BeginTick`))

(fn `UserConstructionScript`)